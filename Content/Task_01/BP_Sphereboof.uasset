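; Test-style sphere actor that fades in and out, shifts vertically and glows in response to numpad keys.
; Construction creates a colored dynamic material instance, and BeginPlay enables input, stores the starting height and hides the sphere.
; Separate timelines drive opacity, rise, return toward origin and emissive glow, which plays or reverses.
; Appear and disappear each stop the opposing movement timeline, offsetting from current height so interrupted motion continues smoothly.
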(event Custom|ChangeOpacity
  (params (Appear :type Boolean))
  (bind (_direction _newtrack_0) (Timeline|Timeline PlayFromStart)
    (:Update
      (Rendering|Material|SetScalarParameterValue (Variables|Default|GetDynamicMaterial) "Opacity" (select Appear (* _newtrack_0 (Variables|Default|GetShowAnimPlayRate)) (- (Math|Float|MakeLiteralFloat 1.0) (* _newtrack_0 (Variables|Default|GetShowAnimPlayRate)))) :!class /Script/Engine.MaterialInstanceDynamic)
      (if (Utilities|Select :Index _direction :Forward (>= _newtrack_0 1.0) :Backward (<= _newtrack_0 0.0))
        (Timeline|Timeline Stop)))))

(event Custom|Dissapear
  (bind _returnvalue (Transformation|GetActorLocation))
  (Variables|Default|SetOriginZ_dop (.z (Transformation|GetActorLocation)))
  (bind _newtrack_0 (Timeline|Timeline_1 PlayFromStart)
    (:Update
      (Transformation|SetActorLocation (Math|Vector|MakeVector (.x _returnvalue) (.y _returnvalue) (+ (Variables|Default|GetOriginZ_dop) (* _newtrack_0 (Variables|Default|GetShowAnimPlayRate) (Variables|Default|GetDeltaZ) 1.0))) false false)
      (if (select false (>= (.z _returnvalue) (+ (Variables|Default|GetOriginZ) (Variables|Default|GetDeltaZ))) (<= (.z _returnvalue) (Variables|Default|GetOriginZ)))
        (Timeline|Timeline_1 Stop)))))

(event Custom|ChangeZ
  (params (Increase :type Boolean))
  (bind _returnvalue (Transformation|GetActorLocation))
  (bind _deltaz (Variables|Default|GetDeltaZ))
  (Variables|Default|SetIsBusy true)
  (Variables|Default|SetOriginZ_dop (.z (Transformation|GetActorLocation)))
  (bind _newtrack_0 (Timeline|Timeline_0 PlayFromStart)
    (:Update
      (Transformation|SetActorLocation (Math|Vector|MakeVector (.x _returnvalue) (.y _returnvalue) (+ (Variables|Default|GetOriginZ_dop) (* _newtrack_0 (Variables|Default|GetShowAnimPlayRate) (Variables|Default|GetDeltaZ) (select Increase 1.0 -1.0)))) false false)
      (if (select Increase (>= (.z _returnvalue) (+ (Variables|Default|GetOriginZ) _deltaz)) (<= (.z _returnvalue) (- (Variables|Default|GetOriginZ) _deltaz)))
        (Variables|Default|SetIsBusy false)
        (Timeline|Timeline_0 Stop)))
    (:Finished
      (Variables|Default|SetIsBusy false))))

(event Custom|StopMovingDown
  (bind _returnvalue (Transformation|GetActorLocation))
  (bind _newtrack_0 (Timeline|Timeline_1 Stop)
    (:Update
      (Transformation|SetActorLocation (Math|Vector|MakeVector (.x _returnvalue) (.y _returnvalue) (+ (Variables|Default|GetOriginZ_dop) (* _newtrack_0 (Variables|Default|GetShowAnimPlayRate) (Variables|Default|GetDeltaZ) 1.0))) false false)
      (if (select false (>= (.z _returnvalue) (+ (Variables|Default|GetOriginZ) (Variables|Default|GetDeltaZ))) (<= (.z _returnvalue) (Variables|Default|GetOriginZ)))
        (Timeline|Timeline_1 Stop)))))

(event Custom|StopMovingUp
  (bind _returnvalue (Transformation|GetActorLocation))
  (bind _deltaz (Variables|Default|GetDeltaZ))
  (bind _newtrack_0 (Timeline|Timeline_0 Stop)
    (:Update
      (Transformation|SetActorLocation (Math|Vector|MakeVector (.x _returnvalue) (.y _returnvalue) (+ (Variables|Default|GetOriginZ_dop) (* _newtrack_0 (Variables|Default|GetShowAnimPlayRate) (Variables|Default|GetDeltaZ) (select (stale Custom|ChangeZ Increase) 1.0 -1.0)))) false false)
      (if (select (stale Custom|ChangeZ Increase) (>= (.z _returnvalue) (+ (Variables|Default|GetOriginZ) _deltaz)) (<= (.z _returnvalue) (- (Variables|Default|GetOriginZ) _deltaz)))
        (Variables|Default|SetIsBusy false)
        (Timeline|Timeline_0 Stop)))
    (:Finished
      (Variables|Default|SetIsBusy false))))

(event EventBeginPlay
  (Input|EnableInput (Game|GetPlayerController 0))
  (Variables|Default|SetOriginZ (.Z (Math|Vector|BreakVector (Transformation|GetActorLocation))))
  (Rendering|Material|SetScalarParameterValue (Variables|Default|GetDynamicMaterial) "Opacity" 0.0 :!class /Script/Engine.MaterialInstanceDynamic))

(event Collision|EventActorBeginOverlap
  (params (OtherActor :type Actor%20Object%20Reference)))

(event EventTick
  (params (DeltaSeconds :type Float%20%28single-precision%29)))

(event Input|KeyboardEvents|NumPadZero
  (params (Key :type Key%20Structure :default "None"))
  (:Pressed
    (CallFunction|ChangeOpacity true)
    (CallFunction|ChangeZ true)
    (CallFunction|StopMovingDown)))

(event Input|KeyboardEvents|NumPadOne
  (params (Key :type Key%20Structure :default "None"))
  (:Pressed
    (CallFunction|ChangeOpacity false)
    (CallFunction|Dissapear)
    (CallFunction|StopMovingUp)))

(event Input|KeyboardEvents|NumPadTwo
  (params (Key :type Key%20Structure :default "None"))
  (:Pressed
    (bind _newtrack_0 (Timeline|Timeline_2 Play)
      (:Update
        (Rendering|Material|SetScalarParameterValue (Variables|Default|GetDynamicMaterial) "Emissive" (* (Variables|Default|GetMaxEmissive) _newtrack_0) :!class /Script/Engine.MaterialInstanceDynamic)))))

(event Input|KeyboardEvents|NumPadThree
  (params (Key :type Key%20Structure :default "None"))
  (:Pressed
    (bind _newtrack_0 (Timeline|Timeline_2 Reverse)
      (:Update
        (Rendering|Material|SetScalarParameterValue (Variables|Default|GetDynamicMaterial) "Emissive" (* (Variables|Default|GetMaxEmissive) _newtrack_0) :!class /Script/Engine.MaterialInstanceDynamic)))))

(fn ConstructionScript
  (bind _returnvalue (Rendering|Material|CreateDynamicMaterialInstance (Variables|Default|GetSphere) 0 "/Game/Task_01/Materials/M_Sphere_Inst.M_Sphere_Inst" "None" :!class /Script/Engine.PrimitiveComponent))
  (bind _output_get (Variables|Default|SetDynamicMaterial _returnvalue))
  (Rendering|Material|SetVectorParameterValue _output_get "Color" (Variables|Default|GetSphereColor) :!class /Script/Engine.MaterialInstanceDynamic)
  (Rendering|Material|SetScalarParameterValue (Variables|Default|GetDynamicMaterial) "Opacity" 1.0 :!class /Script/Engine.MaterialInstanceDynamic))