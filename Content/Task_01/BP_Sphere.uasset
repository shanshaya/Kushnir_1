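; BP_Sphere is a test actor whose height, opacity and emissive glow are driven by numpad keys.
; The construction script creates a colored dynamic material, and timelines animate its Opacity and Emissive parameters.
; Raise and lower timelines move the actor within a DeltaZ range above its start height, each stopping the other first.
; An optional text render displays DeltaZ and the animation speed on BeginPlay.
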(event Custom|ChangeOpacity
  (params (Appear :type Boolean))
  ;[1 1 1] MaterialParametres
  (bind (_direction _newtrack_0) (Timeline|Timeline PlayFromStart)
    (:Update
      (Rendering|Material|SetScalarParameterValue (Variables|Default|GetDynamicMaterial) "Opacity" (select Appear (* _newtrack_0 1.0) (- (Math|Float|MakeLiteralFloat 1.0) (* _newtrack_0 1.0))) :!class /Script/Engine.MaterialInstanceDynamic)
      (if (Utilities|Select :Index _direction :Forward (>= _newtrack_0 1.0) :Backward (<= _newtrack_0 0.0))
        (Timeline|Timeline Stop)))))

(event Custom|AddEmissive
  ;[1 1 1] MaterialParametres
  (bind _newtrack_0 (Timeline|Timeline_2 Play)
    (:Update
      (Rendering|Material|SetScalarParameterValue (Variables|Default|GetDynamicMaterial) "Emissive" (* (Variables|Default|GetMaxEmissive) _newtrack_0) :!class /Script/Engine.MaterialInstanceDynamic))))

(event Custom|DecreaseEmissive
  ;[1 1 1] MaterialParametres
  (bind _newtrack_0 (Timeline|Timeline_2 Reverse)
    (:Update
      (Rendering|Material|SetScalarParameterValue (Variables|Default|GetDynamicMaterial) "Emissive" (* (Variables|Default|GetMaxEmissive) _newtrack_0) :!class /Script/Engine.MaterialInstanceDynamic))))

(event Custom|DecreaseZ
  (bind _returnvalue (Transformation|GetActorLocation))
  ;[1 1 1] MovingUpAndDown
  (CallFunction|StopMovingUp)
  (Components|Timeline|SetPlayRate (Variables|Default|GetTimeline_1) (Variables|Default|GetShowAnimPlayRate))
  (Variables|Default|SetOriginZ_dop (.z (Transformation|GetActorLocation)))
  (bind _newtrack_0 (Timeline|Timeline_1 PlayFromStart)
    (:Update
      (Transformation|SetActorLocation (Math|Vector|MakeVector (.x _returnvalue) (.y _returnvalue) (+ (Variables|Default|GetOriginZ_dop) (* _newtrack_0 1.0 (Variables|Default|GetDeltaZ) 1.0))) false false)
      (if (select false (>= (.z _returnvalue) (+ (Variables|Default|GetOriginZ) (Variables|Default|GetDeltaZ))) (<= (.z _returnvalue) (Variables|Default|GetOriginZ)))
        (Timeline|Timeline_1 Stop)))))

(event Custom|IncreaseZ
  (bind _returnvalue (Transformation|GetActorLocation))
  ;[1 1 1] MovingUpAndDown
  (CallFunction|StopMovingDown)
  (Components|Timeline|SetPlayRate (Variables|Default|GetUpTimeline) (Variables|Default|GetShowAnimPlayRate))
  (Variables|Default|SetOriginZ_dop (.z (Transformation|GetActorLocation)))
  (bind _newtrack_0 (Timeline|UpTimeline PlayFromStart)
    (:Update
      (Transformation|SetActorLocation (Math|Vector|MakeVector (.x _returnvalue) (.y _returnvalue) (+ (Variables|Default|GetOriginZ_dop) (* _newtrack_0 (Variables|Default|GetDeltaZ)))) false false)
      (if (>= (.z _returnvalue) (+ (Variables|Default|GetOriginZ) (Variables|Default|GetDeltaZ)))
        (Timeline|UpTimeline Stop)))))

(event Custom|StopMovingDown
  (bind _returnvalue (Transformation|GetActorLocation))
  ;[1 1 1] MovingUpAndDown
  (bind _newtrack_0 (Timeline|Timeline_1 Stop)
    (:Update
      (Transformation|SetActorLocation (Math|Vector|MakeVector (.x _returnvalue) (.y _returnvalue) (+ (Variables|Default|GetOriginZ_dop) (* _newtrack_0 1.0 (Variables|Default|GetDeltaZ) 1.0))) false false)
      (if (select false (>= (.z _returnvalue) (+ (Variables|Default|GetOriginZ) (Variables|Default|GetDeltaZ))) (<= (.z _returnvalue) (Variables|Default|GetOriginZ)))
        (Timeline|Timeline_1 Stop)))))

(event Custom|StopMovingUp
  (bind _returnvalue (Transformation|GetActorLocation))
  ;[1 1 1] MovingUpAndDown
  (bind _newtrack_0 (Timeline|UpTimeline Stop)
    (:Update
      (Transformation|SetActorLocation (Math|Vector|MakeVector (.x _returnvalue) (.y _returnvalue) (+ (Variables|Default|GetOriginZ_dop) (* _newtrack_0 (Variables|Default|GetDeltaZ)))) false false)
      (if (>= (.z _returnvalue) (+ (Variables|Default|GetOriginZ) (Variables|Default|GetDeltaZ)))
        (Timeline|UpTimeline Stop)))))

(event EventBeginPlay
  (Variables|Default|SetOriginZ (.Z (Math|Vector|BreakVector (Transformation|GetActorLocation))))
  (bind _textrenderinfo (Variables|Default|GetTextRenderInfo)
    (:then
      (Rendering|Components|TextRender|SetText (Variables|/Script/Engine.TextRenderActor|GetTextRender _textrenderinfo) (Utilities|Text|MakeLiteralText (Utilities|Text|ToText(String) (Utilities|String|Append "Delta Z: " (Utilities|String|ToString(Float) (Variables|Default|GetDeltaZ)) " 
" "Speed: " (Utilities|String|ToString(Float) (Variables|Default|GetShowAnimPlayRate)))))))
    (:else)))

(event Collision|EventActorBeginOverlap
  (params (OtherActor :type Actor%20Object%20Reference)))

(event EventTick
  (params (DeltaSeconds :type Float%20%28single-precision%29)))

(event Input|KeyboardEvents|NumPadZero
  (params (Key :type Key%20Structure :default "None"))
  ;[1 1 1] Input
  (:Pressed
    (CallFunction|ChangeOpacity true)
    (CallFunction|Increasez)))

(event Input|KeyboardEvents|NumPadOne
  (params (Key :type Key%20Structure :default "None"))
  ;[1 1 1] Input
  (:Pressed
    (CallFunction|ChangeOpacity false)
    (CallFunction|DecreaseZ)))

(event Input|KeyboardEvents|NumPadTwo
  (params (Key :type Key%20Structure :default "None"))
  ;[1 1 1] Input
  (:Pressed
    (CallFunction|AddEmissive)))

(event Input|KeyboardEvents|NumPadThree
  (params (Key :type Key%20Structure :default "None"))
  ;[1 1 1] Input
  (:Pressed
    (CallFunction|DecreaseEmissive)))

(fn ConstructionScript
  (bind _returnvalue (Rendering|Material|CreateDynamicMaterialInstance (Variables|Default|GetSphere) 0 "/Game/Task_01/Materials/M_Sphere_Inst.M_Sphere_Inst" "None" :!class /Script/Engine.PrimitiveComponent))
  (bind _output_get (Variables|Default|SetDynamicMaterial _returnvalue))
  (Rendering|Material|SetVectorParameterValue _output_get "Color" (Variables|Default|GetSphereColor) :!class /Script/Engine.MaterialInstanceDynamic))