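; BP_TestEffect is an effect actor that fades a set of lights in and out through its ShowLights and HideLights events.
; On BeginPlay it enables player input and caches the starting intensity of each entry in Lights into a parallel LightsIntensity array.
; A single Timeline plays forward or in reverse, scaling each cached intensity by its track value on every update.
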(event Custom|ShowLights
  (bind _newtrack_0 (Timeline|Timeline PlayFromStart)
    (:Update
      (for (_array_element _array_index) (Variables|Default|GetLights)
        (Rendering|Components|Light|SetIntensity (Variables|/Script/Engine.Light|GetLightComponent _array_element) (* _newtrack_0 (Utilities|Array|Get(acopy) (Variables|Default|GetLights_Intensity) _array_index)))))))

(event Custom|HideLights
  (bind _newtrack_0 (Timeline|Timeline ReverseFromEnd)
    (:Update
      (for (_array_element _array_index) (Variables|Default|GetLights)
        (Rendering|Components|Light|SetIntensity (Variables|/Script/Engine.Light|GetLightComponent _array_element) (* _newtrack_0 (Utilities|Array|Get(acopy) (Variables|Default|GetLights_Intensity) _array_index)))))))

(event EventBeginPlay
  (Input|EnableInput (Game|GetPlayerController 0))
  (for _array_element (Variables|Default|GetLights)
    (Utilities|Array|Add (Variables|Default|GetLights_Intensity) (Variables|/Script/Engine.LightComponentBase|GetIntensity (Variables|/Script/Engine.Light|GetLightComponent _array_element)))))

(event Collision|EventActorBeginOverlap
  (params (OtherActor :type Actor%20Object%20Reference)))

(fn ConstructionScript)