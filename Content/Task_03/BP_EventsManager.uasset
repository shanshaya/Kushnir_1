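; Events manager that triggers named events on BP_TestEffect actors, gathered at BeginPlay, from a semicolon-delimited command string.
; DecodeEventString reads effect name, event and speed by position, ignoring key names.
; FindTargetEffect matches the name against static mesh names, keeping the previous target when none matches.
; ExecuteEvent then sets that actor's timeline play rate and calls the event through a short timer-by-function-name.
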(event Custom|ExecuteEvent
  (params (EventString :type String))
  (bind (_effectname _eventname _speed) (CallFunction|DecodeEventString EventString))
  (CallFunction|FindTargetEffect _effectname)
  (bind _targettesteffectref (Variables|Default|GetTargetTestEffectRef)
    (:then
      (Components|Timeline|SetPlayRate (Variables|/Game/Task_03/BP_TestEffect.BP_TestEffect_C|GetTimeline _targettesteffectref) _speed)
      (Utilities|Time|SetTimerbyFunctionName (Variables|Default|GetTargetTestEffectRef) _eventname 0.1))
    (:else)))

(event EventBeginPlay
  (bind _outactors (Actor|GetAllActorsOfClass "/Game/Task_03/BP_TestEffect.BP_TestEffect_C"))
  (Variables|Default|SetTestEffects _outactors))

(fn ConstructionScript)

(fn DecodeEventString
  (params (InputString :type String))
  (bind _output (LocalVariables|GetOutput))
  (bind _output_get (LocalVariables|SetInputStr InputString))
  (LocalVariables|SetInputStr (Utilities|String|Append _output_get ";"))
  (Utilities|FlowControl|Sequence
    (:then_0
      ;[0.4547 1 0.9402 0.542] ParseString
      (while (not (Utilities|Array|IsEmpty (LocalVariables|GetInputStr))) :!label _label
        (LocalVariables|SetEffectNameOut (Utilities|String|GetSubstring (LocalVariables|GetInputStr) (+ (Utilities|String|FindSubstring (LocalVariables|GetInputStr) ":") 1) (- (Utilities|String|FindSubstring (LocalVariables|GetInputStr) ";") (+ (Utilities|String|FindSubstring (LocalVariables|GetInputStr) ":") 1))))
        (Utilities|Array|Add (LocalVariables|GetOutput) (Utilities|String|GetSubstring (LocalVariables|GetInputStr) (+ (Utilities|String|FindSubstring (LocalVariables|GetInputStr) ":") 1) (- (Utilities|String|FindSubstring (LocalVariables|GetInputStr) ";") (+ (Utilities|String|FindSubstring (LocalVariables|GetInputStr) ":") 1))))
        (LocalVariables|SetInputStr (Utilities|String|RightChop (LocalVariables|GetInputStr) (+ (Utilities|String|FindSubstring (LocalVariables|GetInputStr) ";") 1)))
        (goto _label)))
    (:then_1
      (return (Utilities|Array|Get(acopy) _output) (Utilities|Array|Get(acopy) _output 1) (Math|Conversions|ToFloat(Integer) (Utilities|Array|Get(acopy) _output 2))))))

(fn FindTargetEffect
  (params (Name :type String))
  (bind _array_element (Utilities|Array|ForEachLoopwithBreak (Variables|Default|GetTestEffects) :!label _label)
    (:LoopBody
      (if (Utilities|Enum|Equal(Enum) (Utilities|GetDisplayName (Variables|/Script/Engine.StaticMeshComponent|GetStaticMesh (Variables|/Game/Task_03/BP_TestEffect.BP_TestEffect_C|GetStaticMesh _array_element))) Name)
        (Variables|Default|SetTargetTestEffectRef _array_element)
        (goto _label Break)))))