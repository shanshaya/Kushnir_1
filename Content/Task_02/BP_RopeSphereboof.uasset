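; Test actor for a sphere on an adjustable rope, built from a Cable and a Physics Constraint.
; Mouse wheel and an input axis change the cable length and match the constraint's Z limit to it.
; Keys enable sphere physics, push it or set Speed.
; A callable timeline event resizes the rope, stopping outside fixed bounds; Tick holds gated length interpolation, and several timer and resize calls are disconnected.
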(event Custom|CustomEvent
  (Physics|AddImpulse (Variables|Default|GetSphere) "200.000000,0.000000,0.000000" "None" true))

(event Custom|ChangeRopeLength
  (params (TargetLength :type Float%20%28double-precision%29) (Speed :type Float%20%28double-precision%29))
  (Physics|SetSimulatePhysics (Variables|Default|GetSphere) true)
  (bind _output_get (Variables|Default|SetCurrent%20Cable%20Length (Variables|/Script/CableComponent.CableComponent|GetCableLength (Variables|Default|GetCable))))
  (bind _output_get_2 (Variables|Default|SetDeltaLength (- TargetLength _output_get)))
  (bind _newtrack_0 (Timeline|Timeline_0 PlayFromStart)
    (:Update
      (Class|PhysicsConstraintComponent|SetLinearZLimit (Variables|Default|GetPhysicsConstraint) "LCM_Limited" (+ _output_get (* _newtrack_0 _output_get_2 Speed)))
      (Variables|/Script/CableComponent.CableComponent|SetCableLength (Variables|Default|GetCable) (+ _output_get (* _newtrack_0 _output_get_2 Speed)))
      (if (or (> (+ _output_get (* _newtrack_0 _output_get_2 Speed)) 4e+02) (< (+ _output_get (* _newtrack_0 _output_get_2 Speed)) 5e+01))
        (CallFunction|Stop)))))

(event Custom|Stop
  (bind _newtrack_0 (Timeline|Timeline_0 Stop)
    (:Update
      (Class|PhysicsConstraintComponent|SetLinearZLimit (Variables|Default|GetPhysicsConstraint) "LCM_Limited" (+ (stale Custom|ChangeRopeLength _output_get) (* _newtrack_0 (stale Custom|ChangeRopeLength _output_get_2) (stale Custom|ChangeRopeLength Speed))))
      (Variables|/Script/CableComponent.CableComponent|SetCableLength (Variables|Default|GetCable) (+ (stale Custom|ChangeRopeLength _output_get) (* _newtrack_0 (stale Custom|ChangeRopeLength _output_get_2) (stale Custom|ChangeRopeLength Speed))))
      (if (or (> (+ (stale Custom|ChangeRopeLength _output_get) (* _newtrack_0 (stale Custom|ChangeRopeLength _output_get_2) (stale Custom|ChangeRopeLength Speed))) 4e+02) (< (+ (stale Custom|ChangeRopeLength _output_get) (* _newtrack_0 (stale Custom|ChangeRopeLength _output_get_2) (stale Custom|ChangeRopeLength Speed))) 5e+01))
        (CallFunction|Stop)))))

(event EventBeginPlay
  (Input|EnableInput (Game|GetPlayerController 0)))

(event Collision|EventActorBeginOverlap
  (params (OtherActor :type Actor%20Object%20Reference)))

(event EventTick
  (params (DeltaSeconds :type Float%20%28single-precision%29))
  (bind _cable (Variables|Default|GetCable))
  (Utilities|FlowControl|Gate true
    (:Exit
      (bind _output_get (Variables|/Script/CableComponent.CableComponent|SetCableLength _cable (Math|Interpolation|FInterpTo (Variables|/Script/CableComponent.CableComponent|GetCableLength _cable) 4e+02 DeltaSeconds 1.0)))
      (Class|PhysicsConstraintComponent|SetLinearZLimit (Variables|Default|GetPhysicsConstraint) "LCM_Limited" _output_get))))

(event Input|AxisEvents|InputAxisChangeRopeLength
  (params (AxisValue :type Float%20%28single-precision%29))
  (bind _cable (Variables|Default|GetCable))
  (bind _output_get (Variables|/Script/CableComponent.CableComponent|SetCableLength _cable (+ (Variables|/Script/CableComponent.CableComponent|GetCableLength _cable) AxisValue)))
  (Class|PhysicsConstraintComponent|SetLinearZLimit (Variables|Default|GetPhysicsConstraint) "LCM_Limited" _output_get))

(event Input|MouseEvents|MouseWheelUp
  (params (Key :type Key%20Structure :default "None"))
  (bind _cable (Variables|Default|GetCable))
  (:Pressed
    (bind _output_get (Variables|/Script/CableComponent.CableComponent|SetCableLength _cable (+ (Variables|/Script/CableComponent.CableComponent|GetCableLength _cable) 4e+01)))
    (Class|PhysicsConstraintComponent|SetLinearZLimit (Variables|Default|GetPhysicsConstraint) "LCM_Limited" _output_get)))

(event Input|MouseEvents|LeftMouseButton
  (params (Key :type Key%20Structure :default "None"))
  (:Pressed
    (Physics|AddImpulse (Variables|Default|GetSphere) "200.000000,0.000000,0.000000" "None" true)))

(event Input|MouseEvents|MouseWheelDown
  (params (Key :type Key%20Structure :default "None"))
  (bind _cable (Variables|Default|GetCable))
  (:Pressed
    (bind _output_get (Variables|/Script/CableComponent.CableComponent|SetCableLength _cable (+ (Variables|/Script/CableComponent.CableComponent|GetCableLength _cable) -4e+01)))
    (Class|PhysicsConstraintComponent|SetLinearZLimit (Variables|Default|GetPhysicsConstraint) "LCM_Limited" _output_get)))

(event Input|KeyboardEvents|NumPadFour
  (params (Key :type Key%20Structure :default "None"))
  (:Pressed
    (Physics|SetSimulatePhysics (Variables|Default|GetSphere) true)))

(event Input|KeyboardEvents|NumPadSix
  (params (Key :type Key%20Structure :default "None")))

(event Input|KeyboardEvents|NumPadTwo
  (params (Key :type Key%20Structure :default "None"))
  (:Pressed
    (Variables|Default|SetSpeed 2.0)))

(event Input|KeyboardEvents|NumPadThree
  (params (Key :type Key%20Structure :default "None"))
  (:Pressed
    (Variables|Default|SetSpeed 1.0)))

(fn ConstructionScript)