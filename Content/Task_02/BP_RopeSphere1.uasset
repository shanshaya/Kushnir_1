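; BP_RopeSphere1 is a player-controlled rope-and-sphere actor, a physics sphere with a cable whose length can be changed at runtime.
; On BeginPlay it enables input; numpad keys switch the adjustment speed or turn on sphere physics simulation.
; The ChangeRopeLength axis adjusts the clamped cable length and copies it to the physics constraint's Z linear limit, keeping visual rope and physical constraint in sync.
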(event EventBeginPlay
  (Input|EnableInput (Game|GetPlayerController 0)))

(event Input|AxisEvents|InputAxisChangeRopeLength
  (params (AxisValue :type Float%20%28single-precision%29))
  (bind _cable (Variables|Default|GetCable))
  (bind _output_get (Variables|/Script/CableComponent.CableComponent|SetCableLength _cable (Math|Float|Clamp(Float) (+ (Variables|/Script/CableComponent.CableComponent|GetCableLength _cable) (* AxisValue (Variables|Default|GetSpeed))) 2e+01 4e+02)))
  (Class|PhysicsConstraintComponent|SetLinearZLimit (Variables|Default|GetPhysicsConstraint) "LCM_Limited" _output_get))

(event Input|KeyboardEvents|NumPadFour
  (params (Key :type Key%20Structure :default "None"))
  (:Pressed
    (Physics|SetSimulatePhysics (Variables|Default|GetSphere) true)))

(event Input|KeyboardEvents|NumPadSix
  (params (Key :type Key%20Structure :default "None"))
  (:Pressed
    (Physics|SetSimulatePhysics (Variables|Default|GetSphere) true)))

(event Input|KeyboardEvents|NumPadTwo
  (params (Key :type Key%20Structure :default "None"))
  (:Pressed
    (Variables|Default|SetSpeed 2.0)))

(event Input|KeyboardEvents|NumPadThree
  (params (Key :type Key%20Structure :default "None"))
  (:Pressed
    (Variables|Default|SetSpeed 1.0)))

(fn ConstructionScript)